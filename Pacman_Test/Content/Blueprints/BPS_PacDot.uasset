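; BPS_PacDot is a collectible Pac-Man dot that awards points when the player pawn overlaps it.
; The construction script scales its Sphere by the IsPowerUp flag, so one Blueprint covers normal and power-up dots.
; On overlap with BPS_PacmanPawn, power-ups call EatGhostEvent on the pawn.
; It then adds Points to the Score in BPS_Pacman_TestGameModeBase and destroys itself.
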(event `self.ReceiveBeginPlay`)

(event `self.ReceiveActorBeginOverlap`
  (params (OtherActor :type "Actor Object Reference"))
  (bind _asbps_pacman_pawn (cast `/Game/Blueprints/BPS_PacmanPawn` OtherActor))
  (if (`self.isPowerUp?`)
    (`/Game/Blueprints/BPS_PacmanPawn.EatGhostEvent` _asbps_pacman_pawn))
  (bind _asbps_pacman_test_game_mode_base (cast `/Game/Blueprints/BPS_Pacman_TestGameModeBase` (`GameplayStatics.GetGameMode`)))
  (set `/Game/Blueprints/BPS_Pacman_TestGameModeBase.Score` (+ (`/Game/Blueprints/BPS_Pacman_TestGameModeBase.Score` _asbps_pacman_test_game_mode_base) (`self.Points`)) _asbps_pacman_test_game_mode_base)
  (`self.K2_DestroyActor`))

(fn `UserConstructionScript`
  (if (`self.isPowerUp?`)
    (`SceneComponent.SetWorldScale3D` (`self.Sphere`) (`self.PowerUpScale`))
    (else
      (`SceneComponent.SetWorldScale3D` (`self.Sphere`) (`self.NormalScale`)))))