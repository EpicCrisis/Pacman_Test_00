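; Player Pac-Man pawn that moves one grid cell at a time, eats vulnerable ghosts and dies to deadly ones.
; Tick uses a resettable DoOnce to check walls and gated arrow-key input through game-mode grid lookups, then a timeline lerps each step.
; Eating ghosts awards doubling points until a timer resets the bonus.
; Death costs a life, then reloads the level or resets ghosts and destroys the pawn, triggering a game-mode respawn.
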(event `self.ReceiveBeginPlay`
  ;[1 1 1] Begin Play Event
  (set `self.IsDead?` false)
  (bind _asbps_pacman_test_game_mode_base (cast `/Game/Blueprints/BPS_Pacman_TestGameModeBase` (`GameplayStatics.GetGameMode`)))
  (set `self.GameModeRef` _asbps_pacman_test_game_mode_base)
  (add `self.OnDestroyed` (delegate `RespawnEvent`)))

(event `RespawnEvent` :!signature `self.OnDestroyed`
  (params (DestroyedActor :type "Actor Object Reference"))
  ;[1 1 1] Respawn Pacman
  (`/Game/Blueprints/BPS_Pacman_TestGameModeBase.SpawnPacman` (`self.GameModeRef`)))

(event `GetGhostPoints`
  (bind _gamemoderef (`self.GameModeRef`))
  ;[1 1 1] Add points when eating ghosts.
  (set `/Game/Blueprints/BPS_Pacman_TestGameModeBase.Score` (+ (`/Game/Blueprints/BPS_Pacman_TestGameModeBase.Score` _gamemoderef) (`self.GhostPoints`)) _gamemoderef)
  (set `self.GhostPoints` (* (`self.GhostPoints`) 2))
  (bind _returnvalue (`KismetSystemLibrary.K2_SetTimer` self "ResetBonusPoints" (`self.BonusPointsTime`)))
  (set `self.EatBonusTimerHandle` _returnvalue))

(event `self.ReceiveActorBeginOverlap`
  (params (OtherActor :type "Actor Object Reference"))
  ;[1 1 1] Pacman collide ghost, check if can eat the ghost or not.
  (bind _asbps_ghost_character (cast `/Game/Blueprints/BPS_GhostCharacter` OtherActor))
  (if (and (not (`self.IsDead?`)) (`/Game/Blueprints/BPS_GhostCharacter.CanKill` _asbps_ghost_character))
    (set `self.IsDead?` true)
    (elif (`/Game/Blueprints/BPS_GhostCharacter.CanBeEaten` _asbps_ghost_character)
      (`KismetSystemLibrary.K2_ClearAndInvalidateTimerHandle` (`self.EatBonusTimerHandle`))
      (`self.GetGhostPoints`)
      (`/Game/Blueprints/BPS_GhostCharacter.EatEvent` _asbps_ghost_character))))

(event `ResetBonusPoints`
  ;[1 1 1] Reset the bonus points.
  (set `self.GhostPoints` 200))

(event `EatGhostEvent`
  ;[1 1 1] Pacman causes all ghosts to become vulnerable. (Blue)
  (bind _outactors (`GameplayStatics.GetAllActorsOfClass` "/Game/Blueprints/BPS_GhostCharacter.BPS_GhostCharacter_C"))
  (for _array_element _outactors
    (`/Game/Blueprints/BPS_GhostCharacter.CanBeEatenEvent` _array_element)))

(event `self.ReceiveTick`
  (params (DeltaSeconds :type "Float (single-precision)"))
  (bind _gamemoderef (`self.GameModeRef`))
  ;[1 1 1] Tick Event
  (if (`self.IsDead?`)
    (`/Engine/EditorBlueprintResources/StandardMacros.DoOnce` false
      (:`Completed`
        ;;[1 1 1] Death Sequence
        (`KismetSystemLibrary.Delay` 0.2)
        (`KismetSystemLibrary.PrintString` "YOU DIED" true true (struct :`R` 1.0 :`G` 1.0 :`A` 1.0))
        (`KismetSystemLibrary.Delay` 2.0)
        (bind _result (`/Engine/EditorBlueprintResources/StandardMacros.DecrementInt` (`/Game/Blueprints/BPS_Pacman_TestGameModeBase.Lives` _gamemoderef))
          (:`  `
            (bind _output_get (set `/Game/Blueprints/BPS_Pacman_TestGameModeBase.Lives` _result _gamemoderef))
            (if (== _output_get 0)
              (`KismetSystemLibrary.PrintString` "GAME OVER" true true (struct :`R` 1.0 :`A` 1.0) 5.0)
              (`KismetSystemLibrary.Delay` 5.0)
              (`GameplayStatics.OpenLevel` "Pacman_Level")
              (else
                (bind _outactors (`GameplayStatics.GetAllActorsOfClass` "/Game/Blueprints/BPS_GhostCharacter.BPS_GhostCharacter_C"))
                (for _array_element _outactors
                  (`/Game/Blueprints/BPS_GhostCharacter.ResetLocation` _array_element))
                (`self.K2_DestroyActor`)))))))
    (else
      (`/Engine/EditorBlueprintResources/StandardMacros.DoOnce` false :!label _label
        (:`Completed`
          ;;[1 1 1] Store PacMan Current Location
          (set `self.TempLocation` (`SceneComponent.K2_GetComponentLocation` (`self.DefaultSceneRoot`)))
          ;;[1 1 1] Check Collision
          (bind (_x _y) (`/Game/Blueprints/BPS_Pacman_TestGameModeBase.WorldToGridLocation` (`self.GameModeRef`) (`self.K2_GetActorLocation`)))
          (bind _blockactor (`/Game/Blueprints/BPS_Pacman_TestGameModeBase.GetBlockFromGridLocation` (`self.GameModeRef`) (+ _x 1) _y))
          (if (and (not (`/Game/Blueprints/BPS_GridBlock.isWalkable` _blockactor)) (== (`self.DirectionX`) 1))
            (set `self.DirectionX` 0)
            (else
              (bind (_x_2 _y_2) (`/Game/Blueprints/BPS_Pacman_TestGameModeBase.WorldToGridLocation` (`self.GameModeRef`) (`self.K2_GetActorLocation`)))
              (bind _blockactor_2 (`/Game/Blueprints/BPS_Pacman_TestGameModeBase.GetBlockFromGridLocation` (`self.GameModeRef`) (+ _x_2 -1) _y_2))
              (if (and (not (`/Game/Blueprints/BPS_GridBlock.isWalkable` _blockactor_2)) (== (`self.DirectionX`) -1))
                (set `self.DirectionX` 0)
                (else
                  (bind (_x_3 _y_3) (`/Game/Blueprints/BPS_Pacman_TestGameModeBase.WorldToGridLocation` (`self.GameModeRef`) (`self.K2_GetActorLocation`)))
                  (bind _blockactor_3 (`/Game/Blueprints/BPS_Pacman_TestGameModeBase.GetBlockFromGridLocation` (`self.GameModeRef`) _x_3 (+ _y_3 -1)))
                  (if (and (not (`/Game/Blueprints/BPS_GridBlock.isWalkable` _blockactor_3)) (== (`self.DirectionY`) -1))
                    (set `self.DirectionY` 0)
                    (else
                      (bind (_x_4 _y_4) (`/Game/Blueprints/BPS_Pacman_TestGameModeBase.WorldToGridLocation` (`self.GameModeRef`) (`self.K2_GetActorLocation`)))
                      (bind _blockactor_4 (`/Game/Blueprints/BPS_Pacman_TestGameModeBase.GetBlockFromGridLocation` (`self.GameModeRef`) _x_4 (+ _y_4 1)))
                      (if (and (not (`/Game/Blueprints/BPS_GridBlock.isWalkable` _blockactor_4)) (== (`self.DirectionY`) 1))
                        (set `self.DirectionY` 0))))))))
          ;;[1 1 1] Check Inputs
          (`|ExecutionSequence`
            (:`then_0`
              (`/Engine/EditorBlueprintResources/StandardMacros.Gate` true :!label _label_2
                (:`Exit`
                  (bind (_x_5 _y_5) (`/Game/Blueprints/BPS_Pacman_TestGameModeBase.WorldToGridLocation` (`self.GameModeRef`) (`self.K2_GetActorLocation`)))
                  (bind _blockactor_5 (`/Game/Blueprints/BPS_Pacman_TestGameModeBase.GetBlockFromGridLocation` (`self.GameModeRef`) (+ _x_5 1) _y_5))
                  (if (and (`/Game/Blueprints/BPS_GridBlock.isWalkable` _blockactor_5) (`self.CanChangeDirection`))
                    (set `self.DirectionX` 1)
                    (set `self.DirectionY` 0)
                    ;;[1 1 1] Movement Update
                    (if (or (!= (`self.DirectionX`) 0) (!= (`self.DirectionY`) 0)) :!label _label_3
                      (bind (_direction _movementpercent) (`Timeline|MovementTimeline` :!via `PlayFromStart`)
                        (:`Update`
                          (`SceneComponent.K2_SetWorldLocation` (`self.DefaultSceneRoot`) (`KismetMathLibrary.VLerp` (`self.TempLocation`) (+ (`self.TempLocation`) (`KismetMathLibrary.MakeVector` (* (`self.DirectionX`) 100.0) (* (`self.DirectionY`) 100.0))) _movementpercent) false false))
                        (:`Finished`
                          ;;;[1 1 1] Reset Do Once Event
                          (`self.ResetDoOnce` :!label _label_4)))
                      (else
                        (goto _label_4)))))))
            (:`then_1`
              (`/Engine/EditorBlueprintResources/StandardMacros.Gate` true :!label _label_5
                (:`Exit`
                  (bind (_x_6 _y_6) (`/Game/Blueprints/BPS_Pacman_TestGameModeBase.WorldToGridLocation` (`self.GameModeRef`) (`self.K2_GetActorLocation`)))
                  (bind _blockactor_6 (`/Game/Blueprints/BPS_Pacman_TestGameModeBase.GetBlockFromGridLocation` (`self.GameModeRef`) (+ _x_6 -1) _y_6))
                  (if (and (`/Game/Blueprints/BPS_GridBlock.isWalkable` _blockactor_6) (`self.CanChangeDirection`))
                    (set `self.DirectionX` -1)
                    (set `self.DirectionY` 0)
                    (goto _label_3)))))
            (:`then_2`
              (`/Engine/EditorBlueprintResources/StandardMacros.Gate` true :!label _label_6
                (:`Exit`
                  (bind (_x_7 _y_7) (`/Game/Blueprints/BPS_Pacman_TestGameModeBase.WorldToGridLocation` (`self.GameModeRef`) (`self.K2_GetActorLocation`)))
                  (bind _blockactor_7 (`/Game/Blueprints/BPS_Pacman_TestGameModeBase.GetBlockFromGridLocation` (`self.GameModeRef`) _x_7 (+ _y_7 -1)))
                  (if (and (`/Game/Blueprints/BPS_GridBlock.isWalkable` _blockactor_7) (`self.CanChangeDirection`))
                    (set `self.DirectionY` -1)
                    (set `self.DirectionX` 0)
                    (goto _label_3)))))
            (:`then_3`
              (`/Engine/EditorBlueprintResources/StandardMacros.Gate` true :!label _label_7
                (:`Exit`
                  (bind (_x_8 _y_8) (`/Game/Blueprints/BPS_Pacman_TestGameModeBase.WorldToGridLocation` (`self.GameModeRef`) (`self.K2_GetActorLocation`)))
                  (bind _blockactor_8 (`/Game/Blueprints/BPS_Pacman_TestGameModeBase.GetBlockFromGridLocation` (`self.GameModeRef`) _x_8 (+ _y_8 1)))
                  (if (and (`/Game/Blueprints/BPS_GridBlock.isWalkable` _blockactor_8) (`self.CanChangeDirection`))
                    (set `self.DirectionY` 1)
                    (set `self.DirectionX` 0)
                    (goto _label_3)))))
            (:`then_4`
              (goto _label_3))))))))

(event `Key|Right`
  (params (Key :type "Key Structure"))
  ;[1 1 1] Tick Event
  ;;[1 1 1] Check Inputs
  (:`Pressed`
    (goto _label_2 :!via `Open`))
  (:`Released`
    (goto _label_2 :!via `Close`)))

(event `Key|Left`
  (params (Key :type "Key Structure"))
  ;[1 1 1] Tick Event
  ;;[1 1 1] Check Inputs
  (:`Pressed`
    (goto _label_5 :!via `Open`))
  (:`Released`
    (goto _label_5 :!via `Close`)))

(event `ResetDoOnce`
  ;[1 1 1] Tick Event
  (goto _label :!via `Reset`))

(event `Key|Up`
  (params (Key :type "Key Structure"))
  ;[1 1 1] Tick Event
  ;;[1 1 1] Check Inputs
  (:`Pressed`
    (goto _label_6 :!via `Open`))
  (:`Released`
    (goto _label_6 :!via `Close`)))

(event `Key|Down`
  (params (Key :type "Key Structure"))
  ;[1 1 1] Tick Event
  ;;[1 1 1] Check Inputs
  (:`Pressed`
    (goto _label_7 :!via `Open`))
  (:`Released`
    (goto _label_7 :!via `Close`)))

(fn `UserConstructionScript`)