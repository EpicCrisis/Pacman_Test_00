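; BPS_GhostDestination is a trigger actor that serves as a roaming waypoint for ghosts in the Pacman game.
; When the ghost targeting it overlaps the trigger, it frees itself, clears that ghost's target and asks it to find its next destination.
; It then teleports to a random grid block from the game mode, retrying recursively until the block is walkable.
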(event `self.ReceiveBeginPlay`
  (set `self.isTaken` false))

(event `self.Trigger.OnComponentBeginOverlap`
  (params (OverlappedComponent :type "PrimitiveComponent Object Reference") (OtherActor :type "Actor Object Reference") (OtherComp :type "PrimitiveComponent Object Reference") (OtherBodyIndex :type Integer) (bFromSweep :type Boolean) (SweepResult :type "HitResult Structure (by ref)"))
  (bind _asbps_ghost_character (cast `/Game/Blueprints/BPS_GhostCharacter` OtherActor))
  (if (== (`/Game/Blueprints/BPS_GhostCharacter.CurrentTargetTrigger` _asbps_ghost_character) self)
    (set `self.IsTaken` false)
    (set `/Game/Blueprints/BPS_GhostCharacter.CurrentTargetTrigger` null _asbps_ghost_character)
    (`/Game/Blueprints/BPS_GhostCharacter.FindNextDestination` _asbps_ghost_character)
    (`self.Randomize`)))

(event `Randomize`
  (bind _asbps_pacman_test_game_mode_base (cast `/Game/Blueprints/BPS_Pacman_TestGameModeBase` (`GameplayStatics.GetGameMode`)))
  (bind _output_get (set `self.GameModeRef` _asbps_pacman_test_game_mode_base))
  (bind _blockactor (`/Game/Blueprints/BPS_Pacman_TestGameModeBase.GetBlockFromGridLocation` _output_get (`KismetMathLibrary.RandomIntegerInRange` 0 (- (`/Game/Blueprints/BPS_Pacman_TestGameModeBase.MaxX` _output_get) 1)) (`KismetMathLibrary.RandomIntegerInRange` 0 (- (`/Game/Blueprints/BPS_Pacman_TestGameModeBase.MaxY` _output_get) 1))))
  (if (`/Game/Blueprints/BPS_GridBlock.isWalkable` _blockactor)
    (`self.K2_SetActorLocation` (`self.K2_GetActorLocation` _blockactor) false true)
    (else
      (`self.Randomize`))))

(event `self.ReceiveTick`
  (params (DeltaSeconds :type "Float (single-precision)"))
  ;[1 1 1] Debug to activate randomize.
)

(fn `UserConstructionScript`)