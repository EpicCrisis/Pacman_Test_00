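; Pac-Man ghost character whose GhostType selects its flipbook set and AI movement: Red chases, Pink ambushes ahead of Pac-Man, Cyan and Orange roam random destination actors.
; Timers drive the vulnerable blue, flashing and normal states, while being eaten sends the ghost to its start location.
; Tick picks flipbooks from state and velocity direction.
; AvoidPlayer only prints a proximity message, and RandomBehavior is marked not workable.
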(event `AvoidPlayer`
  ;[1 1 1] Detect if Pacman is too close to ghost when it is blue.
  (if (`self.CanBeEaten`)
    (bind _outactors (`GameplayStatics.GetAllActorsOfClass` "/Game/Blueprints/BPS_PacmanPawn.BPS_PacmanPawn_C"))
    (for _array_element _outactors
      (bind (_returnvalue_x _returnvalue_y) (`KismetMathLibrary.BreakVector` (- (`self.K2_GetActorLocation` _array_element) (`self.K2_GetActorLocation`))))
      (if (or (<= (`KismetMathLibrary.Abs` _returnvalue_x) (`self.AvoidanceDistance`)) (<= (`KismetMathLibrary.Abs` _returnvalue_y) (`self.AvoidanceDistance`)))
        (`KismetSystemLibrary.PrintString` "TOO CLOSE!!!")))))

(event `self.ReceiveBeginPlay`
  ;[1 1 1] BeginPlay, Setup Animation based on colour type
  (set `self.StartLocation` (`self.K2_GetActorLocation`))
  (`self.BackToNormal`)
  (switch `/Game/Blueprints/ENUM_GhostType` (`self.GhostType`)
    (:`NewEnumerator0`
      (setmembers `/Game/Blueprints/Struct_GhostAnimations` :`StructRef` (`self.AnimationStruct`) :`Blue` "/Game/FlipBooks/Blue.Blue" :`Flashing` "/Game/FlipBooks/Flashing_FlipBook.Flashing_FlipBook" :`MoveUp` "/Game/FlipBooks/Red_U.Red_U" :`MoveDown` "/Game/FlipBooks/Red_D.Red_D" :`MoveLeft` "/Game/FlipBooks/Red_L.Red_L" :`MoveRight` "/Game/FlipBooks/Red_R.Red_R" :`Dead_MoveUp` "/Game/FlipBooks/Eyes_UP_Flipbook.Eyes_Up_Flipbook" :`Dead_MoveDown` "/Game/FlipBooks/Eyes_Down_Flipbook.Eyes_Down_Flipbook" :`Dead_MoveLeft` "/Game/FlipBooks/Eyes_Left_Flipbook.Eyes_Left_Flipbook" :`Dead_MoveRight` "/Game/FlipBooks/Eyes_Right_Flipbook.Eyes_Right_Flipbook"))
    (:`NewEnumerator1`
      (setmembers `/Game/Blueprints/Struct_GhostAnimations` :`StructRef` (`self.AnimationStruct`) :`Blue` "/Game/FlipBooks/Blue.Blue" :`Flashing` "/Game/FlipBooks/Flashing_FlipBook.Flashing_FlipBook" :`MoveUp` "/Game/FlipBooks/Pink_U.Pink_U" :`MoveDown` "/Game/FlipBooks/Pink_D.Pink_D" :`MoveLeft` "/Game/FlipBooks/Pink_L.Pink_L" :`MoveRight` "/Game/FlipBooks/Pink_R.Pink_R" :`Dead_MoveUp` "/Game/FlipBooks/Eyes_UP_Flipbook.Eyes_Up_Flipbook" :`Dead_MoveDown` "/Game/FlipBooks/Eyes_Down_Flipbook.Eyes_Down_Flipbook" :`Dead_MoveLeft` "/Game/FlipBooks/Eyes_Left_Flipbook.Eyes_Left_Flipbook" :`Dead_MoveRight` "/Game/FlipBooks/Eyes_Right_Flipbook.Eyes_Right_Flipbook"))
    (:`NewEnumerator2`
      (setmembers `/Game/Blueprints/Struct_GhostAnimations` :`StructRef` (`self.AnimationStruct`) :`Blue` "/Game/FlipBooks/Blue.Blue" :`Flashing` "/Game/FlipBooks/Flashing_FlipBook.Flashing_FlipBook" :`MoveUp` "/Game/FlipBooks/Cyan_U.Cyan_U" :`MoveDown` "/Game/FlipBooks/Cyan_D.Cyan_D" :`MoveLeft` "/Game/FlipBooks/Cyan_L.Cyan_L" :`MoveRight` "/Game/FlipBooks/Cyan_R.Cyan_R" :`Dead_MoveUp` "/Game/FlipBooks/Eyes_UP_Flipbook.Eyes_Up_Flipbook" :`Dead_MoveDown` "/Game/FlipBooks/Eyes_Down_Flipbook.Eyes_Down_Flipbook" :`Dead_MoveLeft` "/Game/FlipBooks/Eyes_Left_Flipbook.Eyes_Left_Flipbook" :`Dead_MoveRight` "/Game/FlipBooks/Eyes_Right_Flipbook.Eyes_Right_Flipbook"))
    (:`NewEnumerator3`
      (setmembers `/Game/Blueprints/Struct_GhostAnimations` :`StructRef` (`self.AnimationStruct`) :`Blue` "/Game/FlipBooks/Blue.Blue" :`Flashing` "/Game/FlipBooks/Flashing_FlipBook.Flashing_FlipBook" :`MoveUp` "/Game/FlipBooks/Orange_U.Orange_U" :`MoveDown` "/Game/FlipBooks/Orange_D.Orange_D" :`MoveLeft` "/Game/FlipBooks/Orange_L.Orange_L" :`MoveRight` "/Game/FlipBooks/Orange_R.Orange_R" :`Dead_MoveUp` "/Game/FlipBooks/Eyes_UP_Flipbook.Eyes_Up_Flipbook" :`Dead_MoveDown` "/Game/FlipBooks/Eyes_Down_Flipbook.Eyes_Down_Flipbook" :`Dead_MoveLeft` "/Game/FlipBooks/Eyes_Left_Flipbook.Eyes_Left_Flipbook" :`Dead_MoveRight` "/Game/FlipBooks/Eyes_Right_Flipbook.Eyes_Right_Flipbook"))))

(event `FindNextDestination`
  ;[1 1 1] Event calls for ghosts of different types to activate movement behaviors. Resets movement trigger.
  (bind _outactors (`GameplayStatics.GetAllActorsOfClass` "/Game/Blueprints/BPS_GhostDestination.BPS_GhostDestination_C"))
  (for _array_element _outactors
    (set `/Game/Blueprints/BPS_GhostDestination.isTaken` false _array_element))
  (switch `/Game/Blueprints/ENUM_GhostType` (`self.GhostType`)
    (:`NewEnumerator0`
      (`self.ChaseEvent`))
    (:`NewEnumerator1`
      (`self.AmbushEvent`))
    (:`NewEnumerator2`
      (`self.RandomMovement` :!label _label))
    (:`NewEnumerator3`
      (goto _label))))

(event `Reset`
  ;[1 1 1] Return Flashing Ghost to Normal Ghost, start hunting.
  (set `self.CanBeEaten` true)
  (set `self.isFlashing` true)
  (`KismetSystemLibrary.Delay` 2.0)
  (`self.BackToNormal`))

(event `EatEvent`
  ;[1 1 1] Event When Pacman Eats This Ghost
  (if (and (`self.CanBeEaten`) (not (`self.IsDead?`)))
    (`KismetSystemLibrary.K2_ClearAndInvalidateTimerHandle` (`self.FlashingEventTimerHandle`))
    (`KismetSystemLibrary.K2_ClearAndInvalidateTimerHandle` (`self.BackToNormalTimerHandle`))
    (set `self.CanBeEaten` false)
    (set `self.IsDead?` true)
    (`NavigationSystem.SimpleMoveToLocation` (`self.GetController`) (`self.StartLocation`))
    (set `CharacterMovementComponent.MaxWalkSpeed` (`self.NormalSpeed`) (`self.CharacterMovement`))))

(event `self.ReceiveTick`
  (params (DeltaSeconds :type "Float (single-precision)"))
  (bind (_animationstruct_blue _animationstruct_flashing _animationstruct_moveup _animationstruct_movedown _animationstruct_moveleft _animationstruct_moveright _animationstruct_dead_moveup _animationstruct_dead_movedown _animationstruct_dead_moveleft) (break `/Game/Blueprints/Struct_GhostAnimations` (`self.AnimationStruct`)))
  (bind (_tempvelocity_x _tempvelocity_y) (`KismetMathLibrary.BreakVector` (`self.TempVelocity`)))
  (bind (_animationstruct_blue_2 _animationstruct_flashing_2) (break `/Game/Blueprints/Struct_GhostAnimations` (`self.AnimationStruct`)))
  (bind (_animationstruct_blue_3 _animationstruct_flashing_3 _animationstruct_moveup_2 _animationstruct_movedown_2 _animationstruct_moveleft_2 _animationstruct_moveright_2 _animationstruct_dead_moveup_2 _animationstruct_dead_movedown_2) (break `/Game/Blueprints/Struct_GhostAnimations` (`self.AnimationStruct`)))
  (bind (_animationstruct_blue_4 _animationstruct_flashing_4 _animationstruct_moveup_3 _animationstruct_movedown_3 _animationstruct_moveleft_3 _animationstruct_moveright_3 _animationstruct_dead_moveup_3) (break `/Game/Blueprints/Struct_GhostAnimations` (`self.AnimationStruct`)))
  (bind _tempvelocity_x_2 (`KismetMathLibrary.BreakVector` (`self.TempVelocity`)))
  (bind (_animationstruct_blue_5 _animationstruct_flashing_5 _animationstruct_moveup_4 _animationstruct_movedown_4 _animationstruct_moveleft_4 _animationstruct_moveright_4 _animationstruct_dead_moveup_4 _animationstruct_dead_movedown_3 _animationstruct_dead_moveleft_2 _animationstruct_dead_moveright) (break `/Game/Blueprints/Struct_GhostAnimations` (`self.AnimationStruct`)))
  (bind (_tempvelocity_x_3 _tempvelocity_y_2) (`KismetMathLibrary.BreakVector` (`self.TempVelocity`)))
  ;[1 1 1] Tick Event
  (if (`self.CanBeEaten`)
    (`PaperFlipbookComponent.SetFlipbook` (`self.SpriteFlipBook`) (select `bool` (`self.isFlashing`) :`false` _animationstruct_blue_2 :`true` _animationstruct_flashing_2))
    (else
      (set `self.TempVelocity` (`self.GetVelocity`))
      (if (> (`KismetMathLibrary.Abs` _tempvelocity_y_2) (- (`MovementComponent.GetMaxSpeed` (`self.CharacterMovement`)) 50.0))
        (if (< _tempvelocity_y 0.0)
          (`PaperFlipbookComponent.SetFlipbook` (`self.SpriteFlipBook`) (select `bool` (`self.IsDead?`) :`false` _animationstruct_moveup_3 :`true` _animationstruct_dead_moveup_3))
          (else
            (`PaperFlipbookComponent.SetFlipbook` (`self.SpriteFlipBook`) (select `bool` (`self.IsDead?`) :`false` _animationstruct_movedown_2 :`true` _animationstruct_dead_movedown_2))))
        (elif (< _tempvelocity_x_2 0.0)
          (`PaperFlipbookComponent.SetFlipbook` (`self.SpriteFlipBook`) (select `bool` (`self.IsDead?`) :`false` _animationstruct_moveleft :`true` _animationstruct_dead_moveleft))
          (else
            (`PaperFlipbookComponent.SetFlipbook` (`self.SpriteFlipBook`) (select `bool` (`self.IsDead?`) :`false` _animationstruct_moveright_4 :`true` _animationstruct_dead_moveright))))))))

(event `CanBeEatenEvent`
  ;[1 1 1] Event When Ghost is Vulnerable(Blue) To Be Eaten By Pacman
  (if (not (`self.IsDead?`))
    (`KismetSystemLibrary.K2_ClearAndInvalidateTimerHandle` (`self.FlashingEventTimerHandle`))
    (`KismetSystemLibrary.K2_ClearAndInvalidateTimerHandle` (`self.BackToNormalTimerHandle`))
    (set `CharacterMovementComponent.MaxWalkSpeed` (`self.BlueSpeed`) (`self.CharacterMovement`))
    (set `self.CanKill` false)
    (set `self.CanBeEaten` true)
    (set `self.isFlashing` false)
    (bind _returnvalue (`KismetSystemLibrary.K2_SetTimer` self "FlashingEvent" (`self.CanBeEatenTime`)))
    (set `self.FlashingEventTimerHandle` _returnvalue)
    (`self.RandomMovement`)))

(event `RandomMovement`
  ;[1 1 1] Move randomly based on triggers.
  (if (not (`self.isDead?`))
    (`/Engine/EditorBlueprintResources/StandardMacros.IsValid` (`self.CurrentTargetTrigger`)
      (:`Is Valid`
        (bind _outactors (`GameplayStatics.GetAllActorsOfClass` "/Game/Blueprints/BPS_GhostDestination.BPS_GhostDestination_C"))
        (set `self.TargetTriggerArray` _outactors)
        (`KismetArrayLibrary.Array_RemoveItem` (`self.TargetTriggerArray`) (`self.CurrentTargetTrigger`)))
      (:`Is Not Valid`
        (bind _outactors_2 (`GameplayStatics.GetAllActorsOfClass` "/Game/Blueprints/BPS_GhostDestination.BPS_GhostDestination_C"))
        (set `self.TargetTriggerArray` _outactors_2)
        (for _array_element (`self.TargetTriggerArray`)
          (if (`/Game/Blueprints/BPS_GhostDestination.isTaken` _array_element)
            (`KismetArrayLibrary.Array_RemoveItem` (`self.TargetTriggerArray`) _array_element)))
        (set `self.CurrentTargetTrigger` (`|GetArrayItem` (`self.TargetTriggerArray`) (`KismetMathLibrary.RandomIntegerInRange` 0 (- (`KismetArrayLibrary.Array_Length` (`self.TargetTriggerArray`)) 1))))
        (set `/Game/Blueprints/BPS_GhostDestination.isTaken` true (`self.CurrentTargetTrigger`))
        (`|AIMoveTo` self (0.0 0.0 0.0) (`self.CurrentTargetTrigger`) 1.0
          (:`OnFail`
            ;;[1 1 1] Stop if dead.
            (`KismetSystemLibrary.Delay` 0.2 :!label _label_2)
            (if (`self.isDead?`)
              (`KismetSystemLibrary.Delay` 0.2)
              (goto _label_2))))))))

(event `FlashingEvent`
  ;[1 1 1] Ghost flashing which allows them to return to normal.
  (set `self.isFlashing` true)
  (bind _returnvalue (`KismetSystemLibrary.K2_SetTimer` self "BackToNormal" (`self.FlashingTime`)))
  (set `self.BackToNormalTimerHandle` _returnvalue))

(event `BackToNormal`
  ;[1 1 1] Return ghost to normal state.
  (set `self.IsDead?` false)
  (set `self.CanBeEaten` false)
  (set `self.isFlashing` false)
  (set `self.CanKill` true)
  (set `CharacterMovementComponent.MaxWalkSpeed` (`self.NormalSpeed`) (`self.CharacterMovement`))
  (`NavMovementComponent.StopActiveMovement` (`self.CharacterMovement`))
  (set `self.CurrentTargetTrigger` null)
  (`self.FindNextDestination`))

(event `ResetLocation`
  ;[1 1 1] Reset the ghosts location.
  (`KismetSystemLibrary.K2_ClearAndInvalidateTimerHandle` (`self.FlashingEventTimerHandle`))
  (`KismetSystemLibrary.K2_ClearAndInvalidateTimerHandle` (`self.BackToNormalTimerHandle`))
  (`self.K2_SetActorLocation` (`self.StartLocation`) false true)
  (set `self.CanKill` false)
  (set `CharacterMovementComponent.MaxWalkSpeed` 0.0 (`self.CharacterMovement`))
  (`self.Reset`))

(event `ChaseEvent`
  ;[1 1 1] Chase Pacman.
  (`|AIMoveTo` self (0.0 0.0 0.0) (`GameplayStatics.GetPlayerController` 0) 1.0
    (:`then`
      (if (not (`self.CanKill`))
        (`self.RandomMovement`)))
    (:`OnFail`
      (`KismetSystemLibrary.Delay` 0.2 :!label _label_3)
      (if (`self.isDead?`)
        (`KismetSystemLibrary.Delay` 0.2)
        (goto _label_3)))))

(event `AmbushEvent`
  (bind (_returnvalue_x _returnvalue_y _returnvalue_z) (`KismetMathLibrary.BreakVector` (`self.K2_GetActorLocation`)))
  (bind _pacmanplayer (`self.PacmanPlayer`))
  (bind _currentambushdistance (`self.CurrentAmbushDistance`))
  (bind (_returnvalue_x_2 _returnvalue_y_2) (`KismetMathLibrary.BreakVector` (`self.K2_GetActorLocation` (`self.PacmanPlayer`))))
  ;[1 1 1] Ambush Pacman by checking the position in front of Pacman's current moving direction.
  (bind _asbps_pacman_pawn (cast `/Game/Blueprints/BPS_PacmanPawn` (`GameplayStatics.GetPlayerPawn` 0)))
  (set `self.PacmanPlayer` _asbps_pacman_pawn)
  (bind _output_get (set `self.AmbushLocation` (`KismetMathLibrary.MakeVector` (+ _returnvalue_x_2 (* (`/Game/Blueprints/BPS_PacmanPawn.DirectionX` _pacmanplayer) _currentambushdistance)) (+ _returnvalue_y_2 (* (`/Game/Blueprints/BPS_PacmanPawn.DirectionY` _pacmanplayer) _currentambushdistance)) _returnvalue_z)))
  (`|AIMoveTo` self _output_get null 1.0
    (:`then`
      (`KismetSystemLibrary.Delay` 1.0)
      (if (`self.CanKill`)
        (`self.AmbushEvent`)
        (else
          (`self.RandomMovement`))))
    (:`OnFail`
      (`KismetSystemLibrary.Delay` 0.2 :!label _label_4)
      (if (`self.isDead?`)
        (`KismetSystemLibrary.Delay` 0.2)
        (goto _label_4)))))

(event `RandomBehavior`
  ;[1 1 1] Erratic behavior change, not workable.
  (`NavMovementComponent.StopActiveMovement` (`self.CharacterMovement`))
  (`self.RandomMovement`)
  (`NavMovementComponent.StopActiveMovement` (`self.CharacterMovement`))
  (`self.ChaseEvent`)
  (`NavMovementComponent.StopActiveMovement` (`self.CharacterMovement`))
  (`self.AmbushEvent`)
  (`self.RandomBehavior`))

(fn `UserConstructionScript`
  (switch `/Game/Blueprints/ENUM_GhostType` (`self.GhostType`)
    (:`NewEnumerator0`
      (`PaperFlipbookComponent.SetFlipbook` (`self.SpriteFlipBook`) "/Game/FlipBooks/Red_U.Red_U"))
    (:`NewEnumerator1`
      (`PaperFlipbookComponent.SetFlipbook` (`self.SpriteFlipBook`) "/Game/FlipBooks/Pink_U.Pink_U"))
    (:`NewEnumerator2`
      (`PaperFlipbookComponent.SetFlipbook` (`self.SpriteFlipBook`) "/Game/FlipBooks/Cyan_U.Cyan_U"))
    (:`NewEnumerator3`
      (`PaperFlipbookComponent.SetFlipbook` (`self.SpriteFlipBook`) "/Game/FlipBooks/Orange_U.Orange_U"))))