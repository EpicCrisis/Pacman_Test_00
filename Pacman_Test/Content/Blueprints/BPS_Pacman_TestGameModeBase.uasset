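; Test game mode for a Pac-Man game that builds the block grid, maps locations to blocks and detects the win.
; BeginPlay spawns grid blocks into an array using a hardcoded row length of 23, rebinding all PacDots' destroy events after each spawn.
; A win message prints when a destroyed dot is the last one found.
; SpawnPacman, not called here, spawns and possesses the pawn at the first PlayerStart.
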(event `self.ReceiveBeginPlay`
  (`self.CreateGrid`))

(event `CreateGrid`
  (`KismetArrayLibrary.Array_Clear` (`self.BlocksArray`))
  (for _index (range (* (`self.MaxX`) (`self.MaxY`)))
    (bind _returnvalue (`|SpawnActorFromClass` "/Game/Blueprints/BPS_GridBlock.BPS_GridBlock_C" (`KismetMathLibrary.MakeTransform` (`KismetMathLibrary.MakeVector` (* (/ _index 23) (`self.Spacing`)) (* (mod _index 23) (`self.Spacing`)))) "AlwaysSpawn" "OverrideRootScale" null null))
    (`KismetArrayLibrary.Array_Add` (`self.BlocksArray`) _returnvalue)
    (bind _outactors (`GameplayStatics.GetAllActorsOfClass` "/Game/Blueprints/BPS_PacDot.BPS_PacDot_C"))
    (for _array_element _outactors
      (add `self.OnDestroyed` _array_element (delegate `WinEvent`)))))

(event `WinEvent` :!signature `self.OnDestroyed`
  (params (DestroyedActor :type "Actor Object Reference"))
  (bind _outactors (`GameplayStatics.GetAllActorsOfClass` "/Game/Blueprints/BPS_PacDot.BPS_PacDot_C"))
  (if (== (`KismetArrayLibrary.Array_Length` _outactors) 1)
    (`KismetSystemLibrary.PrintString` "You Won")))

(event `SpawnPacman`
  (bind _outactors (`GameplayStatics.GetAllActorsOfClass` "/Script/Engine.PlayerStart"))
  (bind _returnvalue (`|SpawnActorFromClass` "/Game/Blueprints/BPS_PacmanPawn.BPS_PacmanPawn_C" (`self.GetTransform` (`|GetArrayItem` _outactors)) "AlwaysSpawn" "OverrideRootScale" null null))
  (`Controller.Possess` (`GameplayStatics.GetPlayerController` 0) _returnvalue))

(fn `GetBlockFromGridLocation`
  (params (X :type Integer) (Y :type Integer))
  (returns (BlockActor :type "/Game/Blueprints/BPS_GridBlock Object Reference"))
  (return (`|GetArrayItem` (`self.BlocksArray`) (+ (* X (`self.MaxX`)) (mod Y (`self.MaxY`))))))

(fn `GetBlockFromWorldLocation`
  (params (Location :type "Vector Structure"))
  (returns (BlockActor :type "/Game/Blueprints/BPS_GridBlock Object Reference"))
  (bind (_x _y) (`self.WorldToGridLocation` Location))
  (bind _blockactor (`self.GetBlockFromGridLocation` _x _y))
  (return _blockactor))

(fn `UserConstructionScript`)

(fn `WorldToGridLocation`
  (params (Location :type "Vector Structure"))
  (returns (X :type Integer) (Y :type Integer))
  (bind _spacing (`self.Spacing`))
  (bind _spacing_2 (`self.Spacing`))
  (return (`KismetMathLibrary.Clamp` (`KismetMathLibrary.FFloor` (/ (+ Location_X (/ _spacing_2 2.0)) _spacing_2)) 0 (- (`self.MaxX`) 1)) (`KismetMathLibrary.Clamp` (`KismetMathLibrary.FFloor` (/ (+ Location_Y (/ _spacing 2.0)) _spacing)) 0 (- (`self.MaxY`) 1))))